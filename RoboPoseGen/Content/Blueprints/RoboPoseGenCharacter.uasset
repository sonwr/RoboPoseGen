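; Character that generates a 2D pose dataset, pairing numbered high-res screenshots with JSON joint labels in a hardcoded folder.
; A looping timer pauses the mesh animation and projects every socket, plus a nose point offset from the head, to screen space.
; While AugmentationBlueprint's AnimationStopped is false, it saves the pair, waits, jitters character and main camera, sweeps character yaw back and forth, then resumes animation.
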(event `self.ReceiveBeginPlay`
  (`|ExecutionSequence`
    (:`then_0`
      (set `self.OutputIndex` 1)
      (set `self.InitLocation` (`self.K2_GetActorLocation`)))
    (:`then_1`
      (`KismetSystemLibrary.K2_SetTimerDelegate` (delegate `Capture_Event`) 4.0 true 4.0))
    (:`then_2`
      (bind _outactors (`GameplayStatics.GetAllActorsOfClass` "/Script/Engine.CameraActor"))
      (for _array_element _outactors
        (if (`KismetStringLibrary.Contains` (`KismetSystemLibrary.GetDisplayName` (`CameraActor.CameraComponent` _array_element)) "MainCameraActor")
          (bind _output_get (set `self.CameraActor` _array_element))
          (set `self.CameraLocation` (`self.K2_GetActorLocation` _output_get)))))))

(event `Capture_Event`
  (bind _returnvalue (`GameplayStatics.GetPlayerController` 0))
  (bind _mesh (`self.Mesh`))
  (bind _nosesphere (`self.NoseSphere`))
  (bind _actorrotationz (`self.ActorRotationZ`))
  (bind _cameralocation (`self.CameraLocation`))
  (bind _cameraactor (`self.CameraActor`))
  (bind _jointdata (`self.JointData`))
  (bind _returnvalue_2 (+ (`self.ActorRotationZ`) (`self.ActorRotationZDir`)))
  (bind _returnvalue_3 (`KismetStringLibrary.Concat_StrStr` "d:\\ue5_temp\\saved\\" (`KismetStringLibrary.Conv_IntToString` (`self.OutputIndex`))))
  (bind _returnvalue_4 (+ (`self.InitLocation`) (`KismetMathLibrary.MakeVector` (`KismetMathLibrary.RandomFloatInRange` -20.0 20.0) (`KismetMathLibrary.RandomFloatInRange` -20.0 20.0))))
  (bind (_x _y) (`KismetMathLibrary.BreakVector2D` (`GameplayStatics.ProjectWorldToScreen` _returnvalue (`SceneComponent.K2_GetComponentLocation` _nosesphere))))
  (`SkeletalMeshComponent.Stop` (`self.Mesh`))
  ;[1 1 1] Generate JointStructData
  (`KismetArrayLibrary.Array_Clear` (`self.JointData`))
  (for _array_element (`SceneComponent.GetAllSocketNames` _mesh)
    (bind (_x_2 _y_2) (`KismetMathLibrary.BreakVector2D` (`GameplayStatics.ProjectWorldToScreen` _returnvalue (`SceneComponent.GetSocketLocation` _mesh _array_element))))
    (`KismetArrayLibrary.Array_Add` _jointdata (make `/Game/Blueprints/JointStruct` (`KismetStringLibrary.Conv_NameToString` _array_element) _x_2 _y_2)))
  ;[1 1 1] Create Nose JointStructData
  (`SceneComponent.K2_SetWorldLocation` _nosesphere (+ (`SceneComponent.GetSocketLocation` _mesh "head") (* (`KismetMathLibrary.GetRightVector` (`SceneComponent.GetSocketRotation` _mesh "head")) 13.0)) false false)
  (`KismetArrayLibrary.Array_Add` _jointdata (make `/Game/Blueprints/JointStruct` "nose" _x _y))
  ;[1 1 1] Animation Stopped Check
  (bind _outactors (`GameplayStatics.GetAllActorsOfClass` "/Game/Blueprints/AugmentationBlueprint.AugmentationBlueprint_C"))
  (for _array_element_2 _outactors
    (if (not (`/Game/Blueprints/AugmentationBlueprint.AnimationStopped` _array_element_2))
      ;[1 1 1] File Save
      (bind _outjsonstring (`|StructToJsonString` (make `/Game/Blueprints/JointStructData` (`self.JointData`))))
      (bind _outjsonobject (`JsonBlueprintFunctionLibrary.FromString` _outjsonstring))
      (`|ExecutionSequence`
        (:`then_0`
          (`JsonBlueprintFunctionLibrary.ToFile` _outjsonobject (make `FilePath` (`KismetStringLibrary.Concat_StrStr` _returnvalue_3 ".json")))
          (`AutomationBlueprintFunctionLibrary.TakeHighResScreenshot` 0 0 (`KismetStringLibrary.Concat_StrStr` _returnvalue_3 ".jpg") null)
          (set `self.OutputIndex` (+ (`self.OutputIndex`) 1))
          ;[1 1 1] Actor Rotation & Location
          (`KismetSystemLibrary.Delay` 2.0)
          (`self.K2_SetActorLocation` _returnvalue_4)
          (`|ExecutionSequence`
            (:`then_0`
              (if (> _actorrotationz 280.0)
                (set `self.ActorRotationZDir` -5)))
            (:`then_1`
              (if (< _actorrotationz 100.0)
                (set `self.ActorRotationZDir` 5)))
            (:`then_2`
              (`self.K2_SetActorRotation` (`KismetMathLibrary.MakeRotator` 0.0 0.0 _returnvalue_2))
              (set `self.ActorRotationZ` _returnvalue_2)
              (`self.K2_SetActorLocation` _cameraactor (+ _cameralocation (`KismetMathLibrary.MakeVector` (`KismetMathLibrary.RandomFloatInRange` 0.0 50.0) (`KismetMathLibrary.RandomFloatInRange` -30.0 30.0) (`KismetMathLibrary.RandomFloatInRange` -20.0 20.0))) false true)
              (`self.K2_SetActorRotation` _cameraactor (`KismetMathLibrary.FindLookAtRotation` _cameralocation _returnvalue_4) false)
              (`SkeletalMeshComponent.Play` (`self.Mesh`) false))))))))

(event `self.ReceiveTick`
  (params (DeltaSeconds :type "Float (single-precision)")))

(fn `UserConstructionScript`)